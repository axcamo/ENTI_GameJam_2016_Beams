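; Player controller for a two-element laser shooter that possesses an existing character and eases an aim point toward the mouse each tick.
; Primary and secondary skills share a game-speed-scaled cooldown and fire fire or ice beams as tinted particles along a line trace from the character.
; A beam damages enemies of the opposite element, while hitting a same-element basic enemy replaces it with its Strong variant, carrying over its path points.
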(event Custom|Init
  (params (characterRef :type BP%20Player%20Character%20Object%20Reference) (gameModeRef :type BP%20Game%20Mode%20Object%20Reference))
  ;[0.03649 1 0] Init
  (CallFunction|PossessExistingCharacter characterRef)
  (Variables|Default|SetgameModeRef gameModeRef))

(event EventTick
  (params (DeltaSeconds :type Float%20%28single-precision%29))
  (bind _worldlocation (Game|Player|ConvertMouseLocationToWorldSpace))
  (bind (_x _y) (Math|Vector|BreakVector _worldlocation))
  ;[1 1 1] Mouse Location Update
  (Variables|Default|SetcoolDownCounter (+ (Variables|Default|GetcoolDownCounter) (* DeltaSeconds (Variables|/Game/Blueprints/Game/BP_GameMode.BP_GameMode_C|GetgameSpeed (Variables|Default|GetgameModeRef)))))
  (Variables|Default|SettargetLocation (Math|Vector|Lerp(Vector) (Variables|Default|GettargetLocation) (Math|Vector|MakeVector _x _y 0.0) (* (Variables|Default|GetmouseToTargetSpeed) (Variables|/Game/Blueprints/Game/BP_GameMode.BP_GameMode_C|GetgameSpeed (Variables|Default|GetgameModeRef))))))

(event Input|ActionEvents|InputActionPrimarySkill
  (params (Key :type Key%20Structure :default "AnyKey"))
  ;[1 1 1] Mechanics
  (:Pressed
    (if (>= (Variables|Default|GetcoolDownCounter) (Variables|Default|GetcoolDownMax))
      (Audio|PlaySound2D "/Game/Resources/Audio/FireLaser.FireLaser")
      (CallFunction|ShootLaser "NewEnumerator0")
      (Variables|Default|SetcoolDownCounter 0.0))))

(event Input|ActionEvents|InputActionSecondarySkill
  (params (Key :type Key%20Structure :default "AnyKey"))
  ;[1 1 1] Mechanics
  (:Pressed
    (if (>= (Variables|Default|GetcoolDownCounter) (Variables|Default|GetcoolDownMax))
      (Audio|PlaySound2D "/Game/Resources/Audio/IceLaser.IceLaser")
      (CallFunction|ShootLaser "NewEnumerator1")
      (Variables|Default|SetcoolDownCounter 0.0))))

(fn ConstructionScript)

(fn PossessExistingCharacter
  (params (character :type BP%20Player%20Character%20Object%20Reference))
  (bind _output_get (Variables|Default|SetcontrolledCharacter character))
  (Pawn|Possess _output_get)
  (return))

(fn ShootLaser
  (params (beamType :type ENUM_Element%20Enum))
  (bind _controlledcharacter (Variables|Default|GetcontrolledCharacter))
  (bind _returnvalue (Transformation|GetActorLocation _controlledcharacter))
  (bind _hitactor (CallFunction|GetHitResult))
  (bind _output_get (Variables|Default|SetbeamType beamType))
  (switch Utilities|FlowControl|Switch|SwitchonENUM_Element _output_get
    (:NewEnumerator0
      (Variables|Default|SetcurrentBeamColor (Variables|Default|GetfireBeamColor)))
    (:NewEnumerator1
      (Variables|Default|SetcurrentBeamColor (Variables|Default|GeticeBeamColor))))
  (bind _returnvalue_2 (Effects|SpawnEmitteratLocation "/Game/Resources/ParticleSystems/PS_Beam.PS_Beam" _returnvalue (Math|Rotator|FindLookatRotation _returnvalue (Variables|Default|GettargetLocation))))
  (Effects|Components|ParticleSystem|SetColorParameter _returnvalue_2 "BeamColor" (Variables|Default|GetcurrentBeamColor))
  (Class|ParticleSystemComponent|SetBeamTargetPoint _returnvalue_2 0 (Variables|Default|GettargetLocation))
  (CallFunction|DamageEnemy _hitactor))

(fn DamageEnemy
  (params (hitActor :type Actor%20Object%20Reference))
  (bind _returnvalue (Utilities|GetClass hitActor))
  (bind _gamemoderef (Variables|Default|GetgameModeRef))
  (bind _returnvalue_2 (== _returnvalue "/Game/Blueprints/Enemies/BP_IceEnemy.BP_IceEnemy_C"))
  (bind _returnvalue_3 (== _returnvalue "/Game/Blueprints/Enemies/BP_FireEnemy.BP_FireEnemy_C"))
  (bind _enemycontroller (Variables|/Game/Blueprints/Game/BP_GameMode.BP_GameMode_C|GetenemyController _gamemoderef))
  (bind _enemyspeed (Variables|/Game/Blueprints/Enemies/BP_EnemyController.BP_EnemyController_C|GetenemySpeed _enemycontroller))
  (switch Utilities|FlowControl|Switch|SwitchonENUM_Element (Variables|Default|GetbeamType)
    (:NewEnumerator0
      (Audio|PlaySound2D "/Game/Resources/Audio/FireLaser.FireLaser")
      (if (or _returnvalue_2 (== _returnvalue "/Game/Blueprints/Enemies/BP_IceEnemyStrong.BP_IceEnemyStrong_C"))
        (bind _asbp_enemy (Utilities|Casting|CastToBP_Enemy hitActor))
        (Default|TakeDamage _asbp_enemy "NewEnumerator0" (Variables|Default|Getdamage))
        (elif _returnvalue_3
          (bind _asbp_enemy_2 (Utilities|Casting|CastToBP_Enemy hitActor))
          (bind _returnvalue_4 (Game|SpawnActorfromClass "/Game/Blueprints/Enemies/BP_FireEnemyStrong.BP_FireEnemyStrong_C" (Transformation|GetActorTransform _asbp_enemy_2) "AlwaysSpawn" _asbp_enemy_2 0))
          (Default|Init _returnvalue_4 _enemyspeed)
          (Variables|/Game/Blueprints/Enemies/BP_Enemy.BP_Enemy_C|SetstartPosition _returnvalue_4 (Variables|/Game/Blueprints/Enemies/BP_Enemy.BP_Enemy_C|GetstartPosition _asbp_enemy_2))
          (Variables|/Game/Blueprints/Enemies/BP_Enemy.BP_Enemy_C|SetmovePoint _returnvalue_4 (Variables|/Game/Blueprints/Enemies/BP_Enemy.BP_Enemy_C|GetmovePoint _asbp_enemy_2))
          (Actor|DestroyActor _asbp_enemy_2))))
    (:NewEnumerator1
      (Audio|PlaySound2D "/Game/Resources/Audio/IceLaser.IceLaser")
      (if (or _returnvalue_3 (== _returnvalue "/Game/Blueprints/Enemies/BP_FireEnemyStrong.BP_FireEnemyStrong_C"))
        (bind _asbp_enemy_3 (Utilities|Casting|CastToBP_Enemy hitActor))
        (Default|TakeDamage _asbp_enemy_3 "NewEnumerator1" (Variables|Default|Getdamage))
        (elif _returnvalue_2
          (bind _asbp_enemy_4 (Utilities|Casting|CastToBP_Enemy hitActor))
          (bind _returnvalue_5 (Game|SpawnActorfromClass "/Game/Blueprints/Enemies/BP_IceEnemyStrong.BP_IceEnemyStrong_C" (Transformation|GetActorTransform _asbp_enemy_4) "AlwaysSpawn" _asbp_enemy_4 0))
          (Default|Init _returnvalue_5 _enemyspeed)
          (Variables|/Game/Blueprints/Enemies/BP_Enemy.BP_Enemy_C|SetstartPosition _returnvalue_5 (Variables|/Game/Blueprints/Enemies/BP_Enemy.BP_Enemy_C|GetstartPosition _asbp_enemy_4))
          (Variables|/Game/Blueprints/Enemies/BP_Enemy.BP_Enemy_C|SetmovePoint _returnvalue_5 (Variables|/Game/Blueprints/Enemies/BP_Enemy.BP_Enemy_C|GetmovePoint _asbp_enemy_4))
          (Actor|DestroyActor _asbp_enemy_4))))))

(fn GetHitResult
  (bind _controlledcharacter (Variables|Default|GetcontrolledCharacter))
  (bind _returnvalue (Transformation|GetActorLocation _controlledcharacter))
  (bind (_x _y) (Math|Vector|BreakVector _returnvalue))
  (bind (_outhit _returnvalue_2) (Collision|LineTraceByChannel (Math|Vector|MakeVector _x _y 0.0) (Variables|Default|GettargetLocation) "TraceTypeQuery1" false 0 "None" true "(R=1.000000,G=0.000000,B=0.000000,A=1.000000)" "(R=1.000000,G=1.000000,B=1.000000,A=0.000000)"))
  (if _returnvalue_2
    (Variables|Default|SettargetLocation (.Location (Collision|BreakHitResult _outhit))))
  (return (.HitActor (Collision|BreakHitResult _outhit))))