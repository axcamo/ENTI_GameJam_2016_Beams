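; BP_DarkPoint is a dark point actor that can be diffused while active and reactivates after a cooldown.
; Difuse calls DiffuseEvnt, which, if active, toggles the state, spawns an explosion effect, starts a CdTime timer and passes that time to the DarkPointWidget.
; The timer toggles the state back, and each toggle switches the sprite between active and inactive textures.
; IsActive exposes the current state.
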(event Custom|ReactivateEvnt
  (CallFunction|SwapState))

(event Custom|DiffuseEvnt
  (bind _cdtime (Variables|Default|GetcdTime))
  (if (Variables|Default|Getactive)
    (CallFunction|SwapState)
    (Effects|SpawnEmitteratLocation "/Game/Resources/ParticleSystems/PS_explosion.PS_explosion" (Transformation|GetWorldLocation (Variables|Default|GetDefaultSceneRoot)))
    (Utilities|Time|SetTimerbyEvent (delegate Custom|ReactivateEvnt) _cdtime)
    (Default|SetCD (Variables|Default|Gethud) _cdtime)))

(event EventBeginPlay
  (CallFunction|SetSprites)
  (bind _asdark_point_widget (Utilities|Casting|CastToDarkPointWidget (UserInterface|GetUserWidgetObject (Variables|Default|GetWidget))))
  (Variables|Default|Sethud _asdark_point_widget))

(event Collision|EventActorBeginOverlap
  (params (OtherActor :type Actor%20Object%20Reference)))

(event EventTick
  (params (DeltaSeconds :type Float%20%28single-precision%29)))

(fn ConstructionScript)

(fn IsActive
  (return (Variables|Default|Getactive)))

(fn SetSprites
  (bind _render (Variables|Default|GetRender))
  (if (Variables|Default|Getactive)
    (Rendering|Components|Sprite|SetSprite _render (Variables|Default|GetactiveTexture))
    (else
      (Rendering|Components|Sprite|SetSprite _render (Variables|Default|GetunactiveTexture)))))

(fn SwapState
  (Variables|Default|Setactive (not (Variables|Default|Getactive)))
  (CallFunction|SetSprites))

(fn Difuse
  (CallFunction|DiffuseEvnt))