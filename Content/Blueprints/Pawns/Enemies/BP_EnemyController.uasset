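; BP_EnemyController is the wave spawner that releases timed groups of enemies during play.
; Tick runs a countdown scaled by the game mode's GameSpeed, prints it for debugging, and starts the next wave at zero.
; InitWave resets the countdown from that EnemyWaves entry and spawns each listed class at a random game-mode spawn point.
; The wave index increments without a bounds check.
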(event EventTick
  (params (DeltaSeconds :type Float%20%28single-precision%29))
  (bind _waveindex (Variables|Default|GetwaveIndex))
  (bind _output_get (Variables|Default|Settimer (- (Variables|Default|Gettimer) (* DeltaSeconds (Variables|/Game/Blueprints/Game/BP_GameMode.BP_GameMode_C|GetgameSpeed (Variables|Default|GetgameModeRef))))))
  (Development|PrintString (Utilities|String|ToString(Float) _output_get))
  (if (<= (Variables|Default|Gettimer) 0.0)
    (CallFunction|InitWave _waveindex)
    (Math|Integer|IncrementInt _waveindex)))

(event EventBeginPlay
  (bind _asbp_game_mode (CallFunction|CasttoBPGameMode))
  (Variables|Default|SetgameModeRef _asbp_game_mode))

(fn ConstructionScript)

(fn InitWave
  (params (index :type Integer))
  (bind _enemywaves (Variables|Default|GetenemyWaves))
  (bind _gamemoderef (Variables|Default|GetgameModeRef))
  (bind _item (Utilities|Array|Get(acopy) _enemywaves index))
  (bind _enemyspawnpoints (Variables|/Game/Blueprints/Game/BP_GameMode.BP_GameMode_C|GetenemySpawnPoints _gamemoderef))
  (bind (_time _enemies) (Utilities|Struct|BreakSTRUCT_EnemyWave _item))
  (Variables|Default|Settimer _time)
  (for _array_element _enemies
    (Game|SpawnActorfromClass _array_element (Transformation|GetActorTransform (Utilities|Array|Get(acopy) _enemyspawnpoints (Math|Random|RandomInteger (Utilities|Array|Length _enemyspawnpoints)))) "Undefined" 0 0))
  (return))