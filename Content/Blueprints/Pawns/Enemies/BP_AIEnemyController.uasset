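; AI controller for enemies that can spawn an enemy pawn and take possession of it.
; PossesNewEnemy picks a random class from EnemyClasses and a random spawn point from BP_GameMode's EnemySpawnPoints, then spawns and possesses that enemy.
; PossesExistingEnemy and the construction script are empty.
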(fn ConstructionScript)

(fn PossesExistingEnemy)

(fn PossesNewEnemy
  (bind _enemyclasses (Variables|Default|GetenemyClasses))
  (bind _asbp_game_mode (CallFunction|CasttoBPGameMode))
  (bind _returnvalue (Game|SpawnActorfromClass (Utilities|Array|Get(acopy) _enemyclasses (Math|Random|RandomInteger (Utilities|Array|Length _enemyclasses))) (Transformation|GetActorTransform (Utilities|Array|Get(acopy) (Variables|/Game/Blueprints/Game/BP_GameMode.BP_GameMode_C|GetenemySpawnPoints _asbp_game_mode) (Math|Random|RandomInteger (Utilities|Array|Length (Variables|/Game/Blueprints/Game/BP_GameMode.BP_GameMode_C|GetenemySpawnPoints _asbp_game_mode))))) "Undefined" 0 0))
  (Pawn|Possess _returnvalue))