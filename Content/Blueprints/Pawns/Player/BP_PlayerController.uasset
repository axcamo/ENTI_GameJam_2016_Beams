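; Player controller that possesses an existing character on Init and aims fire and ice beam skills at the mouse.
; Tick eases a target point toward the deprojected mouse position flattened to Z=0, scaled by game-mode speed, and draws a debug trace to it.
; Primary and secondary inputs spawn tinted beam particles from character to target, with no hit or damage logic.
; Character rotation toward the target is present but disconnected.
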(event Custom|Init
  (params (characterRef :type BP%20Player%20Character%20Object%20Reference) (gameModeRef :type BP%20Game%20Mode%20Object%20Reference))
  ;[0.03649 1 0] Init
  (CallFunction|PossessExistingCharacter characterRef)
  (Variables|Default|SetgameModeRef gameModeRef))

(event EventTick
  (params (DeltaSeconds :type Float%20%28single-precision%29))
  (bind _worldlocation (Game|Player|ConvertMouseLocationToWorldSpace))
  (bind (_x _y) (Math|Vector|BreakVector _worldlocation))
  ;[1 1 1] Mouse Location Update
  (bind _output_get (Variables|Default|SettargetLocation (Math|Vector|Lerp(Vector) (Variables|Default|GettargetLocation) (Math|Vector|MakeVector _x _y 0.0) (* (Variables|Default|GetmouseToTargetSpeed) (Variables|/Game/Blueprints/Game/BP_GameMode.BP_GameMode_C|GetgameSpeed (Variables|Default|GetgameModeRef))))))
  (Collision|LineTraceByChannel (Transformation|GetActorLocation (Variables|Default|GetcontrolledCharacter)) _output_get "TraceTypeQuery1" false 0 "ForOneFrame"))

(event Input|ActionEvents|InputActionPrimarySkill
  (params (Key :type Key%20Structure :default "AnyKey"))
  (bind _controlledcharacter (Variables|Default|GetcontrolledCharacter))
  (bind _returnvalue (Transformation|GetActorLocation _controlledcharacter))
  ;[1 1 1] Mechanics
  (:Pressed
    (bind _returnvalue_2 (Effects|SpawnEmitteratLocation "/Game/Resources/ParticleSystems/PS_Beam.PS_Beam" _returnvalue (Math|Rotator|FindLookatRotation _returnvalue (Variables|Default|GettargetLocation))))
    (Effects|Components|ParticleSystem|SetColorParameter _returnvalue_2 "BeamColor" (Variables|Default|GetfireBeamColor))
    (Class|ParticleSystemComponent|SetBeamTargetPoint _returnvalue_2 0 (Variables|Default|GettargetLocation))))

(event Input|ActionEvents|InputActionSecondarySkill
  (params (Key :type Key%20Structure :default "AnyKey"))
  (bind _controlledcharacter (Variables|Default|GetcontrolledCharacter))
  (bind _returnvalue (Transformation|GetActorLocation _controlledcharacter))
  ;[1 1 1] Mechanics
  (:Pressed
    (bind _returnvalue_2 (Effects|SpawnEmitteratLocation "/Game/Resources/ParticleSystems/PS_Beam.PS_Beam" _returnvalue (Math|Rotator|FindLookatRotation _returnvalue (Variables|Default|GettargetLocation))))
    (Effects|Components|ParticleSystem|SetColorParameter _returnvalue_2 "BeamColor" (Variables|Default|GeticeBeamColor))
    (Class|ParticleSystemComponent|SetBeamTargetPoint _returnvalue_2 0 (Variables|Default|GettargetLocation))))

(fn ConstructionScript)

(fn PossessExistingCharacter
  (params (character :type BP%20Player%20Character%20Object%20Reference))
  (bind _output_get (Variables|Default|SetcontrolledCharacter character))
  (Pawn|Possess _output_get)
  (return))