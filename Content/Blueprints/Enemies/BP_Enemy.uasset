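; BP_Enemy is an elemental enemy that homes in on the player character and dies when its health runs out.
; Init caches the game mode and sets Speed; Tick lerps position toward the character at Z=0, scaled by GameSpeed, and faces the movement direction.
; TakeDamage only lowers Hp when fire beams hit ice enemies or ice beams hit fire enemies.
; Tick polls Hp and calls Die to destroy the actor.
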(event Custom|Init
  (params (speed :type Float%20%28single-precision%29))
  (bind _asbp_game_mode (CallFunction|CasttoBPGameMode))
  (Variables|Default|SetgameModeRef _asbp_game_mode)
  (Variables|Default|Setspeed speed))

(event EventTick
  (params (DeltaSeconds :type Float%20%28single-precision%29))
  (bind _returnvalue (Transformation|GetActorLocation))
  (bind _gamemoderef (Variables|Default|GetgameModeRef))
  (bind _speed (Variables|Default|Getspeed))
  (bind _characterref (Variables|/Game/Blueprints/Game/BP_GameMode.BP_GameMode_C|GetcharacterRef _gamemoderef))
  (bind _gamespeed (Variables|/Game/Blueprints/Game/BP_GameMode.BP_GameMode_C|GetgameSpeed _gamemoderef))
  (bind _returnvalue_2 (Transformation|GetActorLocation _characterref))
  (bind _returnvalue_3 (* DeltaSeconds _gamespeed))
  (bind (_x _y) (Math|Vector|BreakVector _returnvalue_2))
  (bind _returnvalue_4 (* _returnvalue_3 _speed))
  (bind _returnvalue_5 (Math|Vector|MakeVector _x _y 0.0))
  (bind _returnvalue_6 (Math|Vector|Lerp(Vector) _returnvalue _returnvalue_5 _returnvalue_4))
  (Transformation|SetActorLocationAndRotation _returnvalue_6 (Math|Rotator|FindLookatRotation _returnvalue _returnvalue_6))
  (if (<= (Variables|Default|Gethp) 0)
    (CallFunction|Die)))

(fn ConstructionScript)

(fn TakeDamage
  (params (beamType :type ENUM_Element%20Enum) (damageTaken :type Integer))
  (bind _myelement (Variables|Default|GetmyElement))
  (switch Utilities|FlowControl|Switch|SwitchonENUM_Element beamType
    (:NewEnumerator0
      (if (Utilities|Enum|Equal(Enum) _myelement "NewEnumerator1")
        (Variables|Default|Sethp (- (Variables|Default|Gethp) damageTaken) :!label _label)))
    (:NewEnumerator1
      (if (Utilities|Enum|Equal(Enum) _myelement "NewEnumerator0")
        (goto _label)))))

(fn Die
  (Actor|DestroyActor))