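; BP_EnemyController runs timed enemy waves from the EnemyWaves array, spawning each enemy at a random GameMode spawn point.
; InitWave copies the wave's enemy list, sends its duration to the HUD and divides that duration into even spawn intervals.
; Tick scales the wave countdown by GameSpeed but advances the spawn timer unscaled, starting the next wave when the countdown expires.
; SpawnWave sets SpawnNextWave past the list's end, but nothing here reads it.
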(event EventTick
  (params (DeltaSeconds :type Float%20%28single-precision%29))
  (bind _waveindex (Variables|Default|GetwaveIndex))
  (Variables|Default|Settimer (- (Variables|Default|Gettimer) (* DeltaSeconds (Variables|/Game/Blueprints/Game/BP_GameMode.BP_GameMode_C|GetgameSpeed (Variables|Default|GetgameModeRef)))))
  (if (<= (Variables|Default|Gettimer) 0.0)
    (CallFunction|InitWave _waveindex)
    (Math|Integer|IncrementInt _waveindex)
    (else
      (bind _output_get (Variables|Default|SetspawnTimer (+ (Variables|Default|GetspawnTimer) (Utilities|Time|GetWorldDeltaSeconds))))
      (if (>= _output_get (Variables|Default|GetspawnTimerMax))
        (CallFunction|SpawnWave)
        (Variables|Default|SetspawnTimer 0.0)))))

(event EventBeginPlay
  (bind _asbp_game_mode (CallFunction|CasttoBPGameMode))
  (Variables|Default|SetgameModeRef _asbp_game_mode))

(fn ConstructionScript)

(fn InitWave
  (params (index :type Integer))
  (bind _enemywaves (Variables|Default|GetenemyWaves))
  (bind _item (Utilities|Array|Get(acopy) _enemywaves index))
  (bind (_time _enemies) (Utilities|Struct|BreakSTRUCT_EnemyWave _item))
  (Variables|Default|SetwaveItemIndex 0)
  (Utilities|Array|Clear (Variables|Default|GetcurrentWaveEnemies))
  (bind _output_get (Variables|Default|Settimer _time))
  (Variables|/Game/Blueprints/UI/BP_HUD.BP_HUD_C|SetmaxTime (Variables|/Game/Blueprints/Game/BP_GameMode.BP_GameMode_C|GetHUDRef (Variables|Default|GetgameModeRef)) _output_get)
  (Variables|Default|SetspawnTimerMax (/ _time (Math|Conversions|ToFloat(Integer) (Utilities|Array|Length _enemies))))
  (for _array_element _enemies
    (Utilities|Array|Add (Variables|Default|GetcurrentWaveEnemies) _array_element))
  (return))

(fn SpawnWave
  (bind _currentwaveenemies (Variables|Default|GetcurrentWaveEnemies))
  (bind _waveitemindex (Variables|Default|GetwaveItemIndex))
  (bind _gamemoderef (Variables|Default|GetgameModeRef))
  (bind _enemyspawnpoints (Variables|/Game/Blueprints/Game/BP_GameMode.BP_GameMode_C|GetenemySpawnPoints _gamemoderef))
  (bind _returnvalue (Game|SpawnActorfromClass (Utilities|Array|Get(acopy) _currentwaveenemies (Variables|Default|GetwaveItemIndex)) (Transformation|GetActorTransform (Utilities|Array|Get(acopy) _enemyspawnpoints (Math|Random|RandomInteger (Utilities|Array|Length _enemyspawnpoints)))) "Undefined" 0 0))
  (Default|Init _returnvalue (Variables|Default|GetenemySpeed))
  (Math|Integer|IncrementInt _waveitemindex
    (:%20%20
      (if (> _waveitemindex (Utilities|Array|Length _currentwaveenemies))
        (Variables|Default|SetspawnNextWave true)))))