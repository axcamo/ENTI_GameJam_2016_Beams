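; Game mode Blueprint that wires up the level's character, player controller, HUD and enemy controller, and tracks a speed modifier.
; Init stores spawn points, dark points and references, initializes the player controller, shows the HUD and starts audio.
; Each Tick, UpdateSpeedModifier lowers a value for each inactive dark point, then prints and returns it, though Tick discards the result.
; Pause nodes are unconnected stubs.
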(event Custom|Init
  (params (characterRef :type BP%20Player%20Character%20Object%20Reference) (enemySpawnPoints :type Array%20of%20Target%20Point%20Object%20References) (darkPoints :type Array%20of%20BP%20Dark%20Point%20Object%20References) (hudRef :type BP%20HUD%20Object%20Reference) (enemyController :type BP%20Enemy%20Controller%20Object%20Reference))
  (Variables|Default|SetenemySpawnPoints enemySpawnPoints)
  (Variables|Default|SetdarkPoints darkPoints)
  (bind _output_get (Variables|Default|SetcharacterRef characterRef))
  (bind _asbp_player_controller (CallFunction|CasttoBPPlayerController))
  (bind _output_get_2 (Variables|Default|SetplayerControllerRef _asbp_player_controller))
  (Default|Init _output_get_2 _output_get self)
  (bind _output_get_3 (Variables|Default|SetHUDRef hudRef))
  (UserInterface|Viewport|AddtoViewport _output_get_3 0)
  (Variables|Default|SetenemyController enemyController)
  (Audio|Components|Audio|Play (Variables|Default|GetAudio) 0.0))

(event EventTick
  (params (DeltaSeconds :type Float%20%28single-precision%29))
  (CallFunction|UpdateSpeedModifier))

(fn ConstructionScript)

(fn UpdateSpeedModifier
  (for _array_element (Variables|Default|GetdarkPoints)
    (bind _isative (Default|IsActive _array_element))
    (if (not _isative)
      (LocalVariables|SetnewValue (- (LocalVariables|GetnewValue) (/ 0.5 (Math|Conversions|ToFloat(Integer) (Utilities|Array|Length (Variables|Default|GetdarkPoints))))))))
  (Development|PrintText (Utilities|Text|ToText(Float) (LocalVariables|GetnewValue) "HalfToEven"))
  (return (LocalVariables|GetnewValue)))